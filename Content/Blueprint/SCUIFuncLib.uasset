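; SCUIFuncLib is a UI function library with a helper that thins out a list of labels by choosing which ones to hide.
; CalcHideLabels walks the labels with a next-show index, keeping the first and then skipping the hide interval between each kept label.
; It returns the skipped labels as the list to hide, and only does this work when the interval is above zero.
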(fn `Calc Hide Labels`
  (params (HideInterval :type Integer) (Labels :type "Array of String"))
  (returns (HideLabels :type "Array of String"))
  (locals (Local_NextShowIndex :type Integer) (Local_HideLabels :type "Array of String"))
  (if (> HideInterval 0)
    (set `local.Local_NextShowIndex` 0)
    (for (_array_element _array_index) Labels
      (if (== (`local.Local_NextShowIndex`) _array_index)
        (set `local.Local_NextShowIndex` (+ (`local.Local_NextShowIndex`) (+ HideInterval 1)))
        (else
          (`KismetArrayLibrary.Array_Add` (`local.Local_HideLabels`) _array_element))))
    (return (`local.Local_HideLabels`))))